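; BP_EnemyController is the enemy AI controller, running BT_Enemy to drive behavior and trigger the player's loss.
; Its sight perception writes seen state and the BP_Hero reference to the Blackboard, playing a danger sound at the pawn on detection.
; Tick refreshes a random reachable location in the Blackboard every frame and shows the HUD's lost screen whenever IsPlayerNearby is set.
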(event OnTargetPerceptionUpdated(Sight)
  (params (Actor :type Actor%20Object%20Reference) (Stimulus :type AI%20Stimulus%20Structure))
  (AI|Components|Blackboard|SetValueasBool (AI|GetBlackboard 0) (Utilities|Name|MakeLiteralName "IsCharacterSeen") (.bsuccessfullysensed Stimulus))
  (bind _asbp_hero (Utilities|Casting|CastToBP_Hero Actor))
  (AI|Components|Blackboard|SetValueasObject (AI|GetBlackboard 0) (Utilities|Name|MakeLiteralName "MainCharacter") _asbp_hero)
  (if (.bsuccessfullysensed Stimulus)
    (Audio|SpawnSoundatLocation "/Game/Sounds/SoundOfDanger.SoundOfDanger" (Transformation|GetActorLocation (Pawn|GetControlledPawn)) "0, 0, 0" 1.0 1.0 0.0 0 0)))

(event EventBeginPlay
  (AI|RunBehaviorTree "/Game/AI/BT_Enemy.BT_Enemy"))

(event EventTick
  (params (DeltaSeconds :type Float%20%28single-precision%29))
  (AI|Components|Blackboard|SetValueasVector (AI|GetBlackboard 0) (Utilities|Name|MakeLiteralName "RandomLocation") (.RandomLocation (AI|Navigation|GetRandomReachablePointinRadius (Transformation|GetActorLocation) 1e+03 0 0)))
  (if (ScalableFloat|GetValueasBool (AI|GetBlackboard 0) (Utilities|Name|MakeLiteralName "IsPlayerNearby"))
    (bind _asbp_my_hud (Utilities|Casting|CastToBP_MyHUD (HUD|GetHUD (Game|GetPlayerController 0))))
    (Default|ShowLostScreen _asbp_my_hud)))

(fn ConstructionScript)
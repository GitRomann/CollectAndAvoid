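; BP_CoinSpawner is an actor that periodically spawns BP_Coin pickups inside a box volume.
; BeginPlay starts a looping timer that calls SpawnCoin every few seconds.
; SpawnCoin places a coin at a random point within the Box component's bounds while CurrentCount is below MaxCount.
; The counter only increments here, so MaxCount caps the total spawned unless something else lowers it.
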(event EventBeginPlay
  (Utilities|Time|SetTimerbyFunctionName 0 "SpawnCoin" 5.0 true))

(event Collision|EventActorBeginOverlap
  (params (OtherActor :type Actor%20Object%20Reference)))

(event EventTick
  (params (DeltaSeconds :type Float%20%28single-precision%29)))

(fn ConstructionScript)

(fn SpawnCoin
  (bind _box (Variables|Default|GetBox))
  (bind (_origin _boxextent) (Collision|GetComponentBounds _box))
  (if (< (Variables|Default|GetCurrentCount) (Variables|Default|GetMaxCount))
    (Game|SpawnActorfromClass "/Game/Blueprint/Objects/BP_Coin.BP_Coin_C" (Math|Transform|MakeTransform (Math|Random|RandomPointinBoundingBox _origin _boxextent) "0, 0, 0" "1.000000,1.000000,1.000000") "Undefined" "MultiplyWithRoot" self 0)
    (Variables|Default|SetCurrentCount (+ (Variables|Default|GetCurrentCount) 1))))
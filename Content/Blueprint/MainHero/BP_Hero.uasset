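; BP_Hero is the player character Blueprint, handling movement, look, jump, sprint and pause through Enhanced Input.
; BeginPlay adds the mapping context, and input actions drive the character's movement and controller rotation.
; Sprint raises walk speed and starts a world-space camera shake on every Triggered event, restoring normal speed on completion.
; Pause toggles game pause, BP_MyHUD's pause screen, input mode and cursor visibility.
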(event Input|EnhancedActionEvents|EnhancedInputActionIA_MyMove
  (params (ActionValue :type Vector%202D%20Structure) (ElapsedSeconds :type Float%20%28double-precision%29) (TriggeredSeconds :type Float%20%28double-precision%29) (InputAction :type Input%20Action%20Object%20Reference :default "/Game/MyInput/IA_MyMove.IA_MyMove"))
  (Pawn|Input|AddMovementInput (Transformation|GetActorForwardVector) (.y ActionValue) false)
  (Pawn|Input|AddMovementInput (Transformation|GetActorRightVector) (.x ActionValue) false))

(event Input|EnhancedActionEvents|EnhancedInputActionIA_MyJump
  (params (ActionValue :type Boolean) (ElapsedSeconds :type Float%20%28double-precision%29) (TriggeredSeconds :type Float%20%28double-precision%29) (InputAction :type Input%20Action%20Object%20Reference :default "/Game/MyInput/IA_MyJump.IA_MyJump"))
  (:Triggered
    (Character|Jump))
  (:Completed
    (Character|StopJumping)))

(event Input|EnhancedActionEvents|EnhancedInputActionIA_MyLook
  (params (ActionValue :type Vector%202D%20Structure) (ElapsedSeconds :type Float%20%28double-precision%29) (TriggeredSeconds :type Float%20%28double-precision%29) (InputAction :type Input%20Action%20Object%20Reference :default "/Game/MyInput/IA_MyLook.IA_MyLook"))
  (Pawn|Input|AddControllerYawInput (.x ActionValue))
  (Pawn|Input|AddControllerPitchInput (.y ActionValue)))

(event Input|EnhancedActionEvents|EnhancedInputActionIA_MySprint
  (params (ActionValue :type Boolean) (ElapsedSeconds :type Float%20%28double-precision%29) (TriggeredSeconds :type Float%20%28double-precision%29) (InputAction :type Input%20Action%20Object%20Reference :default "/Game/MyInput/IA_MySprint.IA_MySprint"))
  (bind _charactermovement (Variables|Character|GetCharacterMovement))
  (:Triggered
    (Variables|Default|SetIsSpriting true)
    (Variables|/Script/Engine.CharacterMovementComponent|SetMaxWalkSpeed _charactermovement 1.5e+03)
    (CameraShakes|StartCameraShake (Variables|/Script/Engine.PlayerController|GetPlayerCameraManager (Game|GetPlayerController 0)) "/Game/Blueprint/MainHero/CameraShake/BP_SprintShake.BP_SprintShake_C" 1.0 "World" "0, 0, 0"))
  (:Completed
    (Variables|Default|SetIsSpriting false)
    (Variables|/Script/Engine.CharacterMovementComponent|SetMaxWalkSpeed _charactermovement 7e+02)))

(event Input|EnhancedActionEvents|EnhancedInputActionIA_Pause
  (params (ActionValue :type Boolean) (ElapsedSeconds :type Float%20%28double-precision%29) (TriggeredSeconds :type Float%20%28double-precision%29) (InputAction :type Input%20Action%20Object%20Reference :default "/Game/MyInput/IA_Pause.IA_Pause"))
  (bind _returnvalue (Game|GetPlayerController 0))
  (:Started
    (bind _asbp_my_hud (Utilities|Casting|CastToBP_MyHUD (HUD|GetHUD _returnvalue)))
    (if (not false)
      (if (Game|IsGamePaused)
        (Input|SetInputModeGameOnly _returnvalue false)
        (Default|HidePauseScreen _asbp_my_hud)
        (Game|SetGamePaused false)
        (Variables|/Script/Engine.PlayerController|SetbShowMouseCursor _returnvalue false)
        (else
          (Input|SetInputModeGameandUI _returnvalue 0 "DoNotLock" true false)
          (Default|ShowPauseScreen _asbp_my_hud)
          (Game|SetGamePaused true)
          (Variables|/Script/Engine.PlayerController|SetbShowMouseCursor _returnvalue true))))))

(event EventBeginPlay
  (Input|AddMappingContext (PlayerController|LocalPlayerSubsystems|GetEnhancedInputLocalPlayerSubsystem (Game|GetPlayerController 0)) "/Game/MyInput/IMC_MyMappingContext.IMC_MyMappingContext" 0 "(bIgnoreAllPressedKeysUntilRelease=True,bForceImmediately=False,bNotifyUserSettings=False)"))

(fn ConstructionScript)